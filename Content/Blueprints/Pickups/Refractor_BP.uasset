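; Refractor pickup that awards Zenny to the ServbotRunner player character.
; On mesh overlap with a ServbotRunner, a timeline moves it toward a point just above the player using VInterpTo plus the timeline's vector offset.
; When the timeline finishes, it adds and counts its Value as Zenny on the player, then plays a sound, spawns an emitter and destroys itself.
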(event OnComponentBeginOverlap(StaticMesh)
  (params (OverlappedComponent :type Primitive%20Component%20Object%20Reference) (OtherActor :type Actor%20Object%20Reference) (OtherComp :type Primitive%20Component%20Object%20Reference) (OtherBodyIndex :type Integer) (bFromSweep :type Boolean) (SweepResult :type Hit%20Result%20Structure%20%28by%20ref%29))
  (bind _returnvalue (Game|GetPlayerCharacter 0))
  (bind _value (Variables|Default|GetValue))
  (bind _returnvalue_2 (Transformation|GetActorLocation _returnvalue))
  (Utilities|Casting|CastToServbotRunner OtherActor)
  (bind _vector (Timeline|Timeline_0 Play)
    (:Update
      (Transformation|SetActorLocation (+ _vector (Math|Interpolation|VInterpTo (Transformation|GetActorLocation) (Math|Vector|MakeVector (.x _returnvalue_2) (.y _returnvalue_2) (+ (.z _returnvalue_2) 4e+01)) (Utilities|Time|GetWorldDeltaSeconds) 1e+01)) false false))
    (:Finished
      (bind _asservbot_runner (Utilities|Casting|CastToServbotRunner (Game|GetPlayerCharacter 0)))
      (Class|Servbot|AddZenny _asservbot_runner _value)
      (Default|CountZenny _asservbot_runner _value)
      (CallFunction|RemoveRefractor))))

(fn ConstructionScript)

(fn RemoveRefractor
  (bind _returnvalue (Transformation|GetActorLocation))
  (Audio|PlaySoundatLocation "/Game/Audio/SFX/sfx-getzenny1.sfx-getzenny1" _returnvalue "0, 0, 0" 1.0 1.0 0.0 0 0 0)
  (Effects|SpawnEmitteratLocation 0 _returnvalue)
  (Actor|DestroyActor))