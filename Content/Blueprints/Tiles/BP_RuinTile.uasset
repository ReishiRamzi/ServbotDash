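; Ruin track tile for the Servbot runner that, when the runner overlaps its end trigger, has the game mode's TileManager add another ruin tile at its attach point.
; The construction script scatters random coins in the CoinArea box as child actors.
; Player Zenny thresholds gate a blocker at one of three spawn points and a rarer random pickup.
; The collectible generation calls are disconnected and never run.
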(event OnComponentBeginOverlap(TileEndTrigger)
  (params (OverlappedComponent :type Primitive%20Component%20Object%20Reference) (OtherActor :type Actor%20Object%20Reference) (OtherComp :type Primitive%20Component%20Object%20Reference) (OtherBodyIndex :type Integer) (bFromSweep :type Boolean) (SweepResult :type Hit%20Result%20Structure%20%28by%20ref%29))
  (Utilities|Casting|CastToServbotRunner OtherActor)
  (bind _asdash_game_mode_bp (Utilities|Casting|CastToDashGameMode_BP (Game|GetGameMode)))
  (Class|TileManager|AddRuinTile (Variables|/Game/Blueprints/Game/DashGameMode_BP.DashGameMode_BP_C|GetTileManager _asdash_game_mode_bp) (Variables|Default|GetSpawnAttachPoint)))

(fn ConstructionScript
  (CallFunction|SetSpawnPoints)
  (CallFunction|SpawnCoins)
  (CallFunction|SpawnBlocker)
  (CallFunction|SpawnPickup))

(fn SetSpawnPoints
  (Variables|Default|SetSpawnPoints (Utilities|Array|MakeArray (Transformation|GetRelativeTransform (Variables|Default|GetSpawnPoint_01)) (Transformation|GetRelativeTransform (Variables|Default|GetSpawnPoint_02)) (Transformation|GetRelativeTransform (Variables|Default|GetSpawnPoint_03)))))

(fn SpawnBlocker
  (bind _spawnpoints (Variables|Default|GetSpawnPoints))
  (bind _asservbot_runner (Utilities|Casting|CastToServbotRunner (Game|GetPlayerCharacter 0)))
  (if (> (Variables|/Script/ServbotDash.Servbot|GetZenny _asservbot_runner) 5000)
    (AddComponent|AddChildActorComponent false (Utilities|Array|Get(acopy) _spawnpoints (Math|Random|RandomIntegerinRange 0 (Utilities|Array|LastIndex _spawnpoints))))))

(fn SpawnCoins
  (bind _coinarea (Variables|Default|GetcoinArea))
  (bind _returnvalue (Transformation|GetRelativeTransform _coinarea))
  (bind _boxextent (Variables|/Script/Engine.BoxComponent|GetBoxExtent _coinarea))
  (bind _returnvalue_2 (Math|Random|RandomPointinBoundingBox (.location _returnvalue) _boxextent))
  (bind _returnvalue_3 (Math|Conversions|ToTransform(Vector) _returnvalue_2))
  (for _index (range 0 (Math|Random|RandomIntegerinRange 3 7))
    (switch int (Math|Random|RandomIntegerinRange 0 3)
      (:Default
        (AddComponent|AddChildActorComponent false _returnvalue_3 :!label _label))
      (:0
        (goto _label))
      (:1
        (AddComponent|AddChildActorComponent false _returnvalue_3))
      (:2
        (AddComponent|AddChildActorComponent false _returnvalue_3))
      (:3
        (AddComponent|AddChildActorComponent false _returnvalue_3)))))

(fn SpawnPickup
  (bind _coinarea (Variables|Default|GetcoinArea))
  (bind _asservbot_runner (Utilities|Casting|CastToServbotRunner (Game|GetPlayerCharacter 0)))
  (if (> (Variables|/Script/ServbotDash.Servbot|GetZenny _asservbot_runner) 10000)
    (if (== (Math|Random|RandomIntegerinRange 0 5) 2)
      (AddComponent|AddChildActorComponent false (Math|Conversions|ToTransform(Vector) (Math|Random|RandomPointinBoundingBox (.location (Transformation|GetRelativeTransform _coinarea)) (Variables|/Script/Engine.BoxComponent|GetBoxExtent _coinarea)))))))

(fn GenerateCollectablesBP
  (bind _spawnarea (Variables|Default|GetSpawnArea))
  (bind _collectabletypes (Variables|Default|GetCollectableTypes))
  (bind _chance (Variables|Default|GetChance))
  (bind _returnvalue (Utilities|Array|Length _collectabletypes))
  (bind _returnvalue_2 (Math|Conversions|ToFloat(Integer) _returnvalue))
  (bind _returnvalue_3 (* _returnvalue_2 1e+02))
  (bind _returnvalue_4 (Math|Float|Truncate _returnvalue_3))
  (bind _returnvalue_5 (Math|Random|RandomIntegerinRange 0 _returnvalue_4))
  (bind _returnvalue_6 (Math|Conversions|ToFloat(Integer) _returnvalue_5))
  (bind _returnvalue_7 (/ _returnvalue_6 _chance))
  (for _index (range 0 9)
    (Development|PrintString (Utilities|String|ToString(Float) _returnvalue_7) true true "(R=0.000000,G=0.660000,B=1.000000,A=1.000000)" 5.0)
    (Game|SpawnActorfromClass (Utilities|Array|Get(acopy) _collectabletypes (Math|Float|Truncate _returnvalue_7)) (Math|Conversions|ToTransform(Vector) (Math|Random|RandomPointinBoundingBox (Transformation|GetWorldLocation _spawnarea) (Variables|/Script/Engine.BoxComponent|GetBoxExtent _spawnarea))) "AdjustIfPossibleButAlwaysSpawn" 0 0)))