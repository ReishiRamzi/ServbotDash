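; AI controller for the Servbot AI pawn, driven by a behavior tree.
; On possession it caches the pawn, sets up the Servbot blackboard, starts the behavior tree and writes the pawn's current location to a blackboard key.
; Walk, Run and Sprint events pass through to the possessed Servbot.
; The perception update event is empty; its target-tracking blackboard writes and a bomb lookup are left disconnected.
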(event OnTargetPerceptionUpdated(AIPerception)
  (params (Actor :type Actor%20Object%20Reference) (Stimulus :type AI%20Stimulus%20Structure)))

(event Custom|Walk
  (Default|Walk (Variables|Default|GetThisServbot)))

(event Custom|Run
  (Default|Run (Variables|Default|GetThisServbot)))

(event Custom|Sprint
  (Default|Sprint (Variables|Default|GetThisServbot)))

(event EventPossess
  (params (PossessedPawn :type Pawn%20Object%20Reference))
  (bind _asservbot_ai_bp (Utilities|Casting|CastToServbot_AI_BP PossessedPawn))
  (Variables|Default|SetThisServbot _asservbot_ai_bp)
  (bind _blackboardcomponent (Class|AIController|UseBlackboard "/Game/Blueprints/AI/Servbot_BB.Servbot_BB"))
  (AI|RunBehaviorTree "/Game/Blueprints/AI/Servbot_AI_BT.Servbot_AI_BT")
  (AI|Components|Blackboard|SetValueasVector _blackboardcomponent (Variables|Default|GetLocationKeyName) (Transformation|GetActorLocation (Pawn|GetControlledPawn))))

(fn ConstructionScript)