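; Behavior tree service that lets a Servbot AI detect nearby objects of a configurable type, intended for bombs going by its name.
; Each AI tick sphere-traces around the pawn, then line-traces to every hit to confirm line of sight, ignoring other Servbots.
; Visible hits set the target actor and location blackboard keys; blocked ones clear the actor, so the last hit wins.
; Debug drawing and printing remain on, and the BP_Bomb cast check is disconnected.
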(event EventReceiveActivationAI
  (params (OwnerController :type AI%20Controller%20Object%20Reference) (ControlledPawn :type Pawn%20Object%20Reference)))

(event EventReceiveTickAI
  (params (OwnerController :type AI%20Controller%20Object%20Reference) (ControlledPawn :type Pawn%20Object%20Reference) (DeltaSeconds :type Float%20%28single-precision%29))
  (if (!= (Variables|Default|GetAIConRef) 0)
    _
    (else
      (bind _asservbot_aicon_bp (Utilities|Casting|CastToServbot_AICon_BP OwnerController))
      (bind _output_get (Variables|Default|SetAIConRef _asservbot_aicon_bp))))
  (bind _outactors (Actor|GetAllActorsOfClass "/Game/Blueprints/AI/Servbot_AI_BP.Servbot_AI_BP_C"))
  (bind _output_get_2 (Variables|Default|SetMyLocation (Transformation|GetActorLocation (Pawn|GetControlledPawn _output_get))))
  (bind _outhits (Collision|MultiSphereTraceForObjects _output_get_2 (+ _output_get_2 "0, 0,15.000000") 1.5e+03 (Variables|Default|GetDesiredObjectType) false _outactors "ForDuration" true "(R=1.000000,G=0.260417,B=0.915319,A=1.000000)" "(R=0.000000,G=1.000000,B=0.000000,A=1.000000)" 2.0))
  (bind _array_element (Utilities|Array|ForEachLoopwithBreak _outhits)
    (:LoopBody
      (bind _outhit (Collision|LineTraceForObjects (Variables|Default|GetMyLocation) (Transformation|GetActorLocation (.HitActor (Collision|BreakHitResult _array_element))) (Variables|Default|GetDesiredObjectType) false _outactors "ForOneFrame"))
      (Development|PrintString (Utilities|GetDisplayName (.HitActor (Collision|BreakHitResult _outhit))))
      (if (== (.HitActor (Collision|BreakHitResult _outhit)) (.HitActor (Collision|BreakHitResult _array_element)))
        (Class|BTFunctionLibrary|SetBlackboardValueasObject (Variables|Default|GetTargetActorKey) (.HitActor (Collision|BreakHitResult _outhit)))
        (AI|BehaviorTree|SetBlackboardValueasVector (Variables|Default|GetTargetLocationKey) (Transformation|GetActorLocation (.HitActor (Collision|BreakHitResult _outhit))))
        (else
          (Class|BTFunctionLibrary|SetBlackboardValueasObject (Variables|Default|GetTargetActorKey)))))))

(event EventTick
  (params (OwnerActor :type Actor%20Object%20Reference) (DeltaSeconds :type Float%20%28single-precision%29)))