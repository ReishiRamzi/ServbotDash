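; Servbot AI character Blueprint that provides movement speed presets and physics-driven animation for the Servbot.
; Walk, Run and Sprint events set fixed max walk speeds on CharacterMovement, while UpdateMoveSpeed applies an arbitrary speed through SetNewMoveSpeed.
; ActivatePhysicalAnimation simulates bodies below a given bone, blending physics with animation via the Servbot physical animation and constraint profiles, hardcoded drive settings and caller-supplied weights.
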(event Custom|UpdateMoveSpeed
  (params (NewSpeed :type Float%20%28single-precision%29))
  (CallFunction|SetNewMoveSpeed NewSpeed))

(event Custom|Walk
  (Variables|Default|SetMovementSpeed 7e+01)
  (Variables|/Script/Engine.CharacterMovementComponent|SetMaxWalkSpeed (Variables|Character|GetCharacterMovement) (stale Custom|Sprint _output_get)))

(event Custom|Run
  (Variables|Default|SetMovementSpeed 3e+02)
  (Variables|/Script/Engine.CharacterMovementComponent|SetMaxWalkSpeed (Variables|Character|GetCharacterMovement) (stale Custom|Sprint _output_get)))

(event Custom|Sprint
  (bind _output_get (Variables|Default|SetMovementSpeed 375.0))
  (Variables|/Script/Engine.CharacterMovementComponent|SetMaxWalkSpeed (Variables|Character|GetCharacterMovement) _output_get))

(fn ConstructionScript)

(fn SetNewMoveSpeed
  (params (NewSpeed :type Float%20%28single-precision%29))
  (Variables|/Script/Engine.CharacterMovementComponent|SetMaxWalkSpeed (Variables|Character|GetCharacterMovement) NewSpeed))

(fn ActivatePhysicalAnimation
  (params (BlendWeight :type Float%20%28single-precision%29) (BlendStrengthWeight :type Float%20%28single-precision%29) (BoneName :type Name) (IncludeSelf :type Boolean))
  (LocalVariables|SetBlendWeightValue BlendWeight)
  (LocalVariables|SetBlendStrengthValue BlendStrengthWeight)
  (LocalVariables|SetBoneNameValue BoneName)
  (LocalVariables|SetbIncludeSelf IncludeSelf)
  (Class|PhysicalAnimationComponent|SetSkeletalMeshComponent (Variables|Default|GetPhysicalAnimation) (Variables|Character|GetMesh))
  (Class|PhysicalAnimationComponent|ApplyPhysicalAnimationProfileBelow (Variables|Default|GetPhysicalAnimation) (LocalVariables|GetBoneNameValue) "Servbot_PhysicalAnimationProfile" (LocalVariables|GetbIncludeSelf) false)
  (Class|PhysicalAnimationComponent|ApplyPhysicalAnimationSettingsBelow (Variables|Default|GetPhysicalAnimation) (LocalVariables|GetBoneNameValue) (Utilities|Struct|MakePhysicalAnimationData true 1e+03 1e+02 1e+03 1e+02) (LocalVariables|GetbIncludeSelf))
  (Class|SkeletalMeshComponent|SetAllBodiesBelowSimulatePhysics (Variables|Character|GetMesh) (LocalVariables|GetBoneNameValue) true (LocalVariables|GetbIncludeSelf))
  (Class|SkeletalMeshComponent|SetAllBodiesBelowPhysicsBlendWeight (Variables|Character|GetMesh) (LocalVariables|GetBoneNameValue) (LocalVariables|GetBlendWeightValue) false (LocalVariables|GetbIncludeSelf))
  (Class|PhysicalAnimationComponent|SetStrengthMultiplyer (Variables|Default|GetPhysicalAnimation) (LocalVariables|GetBlendStrengthValue))
  (Class|SkeletalMeshComponent|SetConstraintProfile (Variables|Character|GetMesh) "None" "Servbot_ConstraintProfile" false))