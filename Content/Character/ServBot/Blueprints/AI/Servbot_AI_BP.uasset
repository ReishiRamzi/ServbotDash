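; Servbot AI character Blueprint that controls how fast the Servbot moves.
; Walk, Run and Sprint events each store a preset MovementSpeed and apply it to the CharacterMovement component's max walk speed.
; UpdateMoveSpeed takes an arbitrary speed and applies it through SetNewMoveSpeed, leaving the stored MovementSpeed unchanged.
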(event Custom|UpdateMoveSpeed
  (params (NewSpeed :type Float%20%28single-precision%29))
  (CallFunction|SetNewMoveSpeed NewSpeed))

(event Custom|Walk
  (Variables|Default|SetMovementSpeed 7e+01)
  (Variables|/Script/Engine.CharacterMovementComponent|SetMaxWalkSpeed (Variables|Character|GetCharacterMovement) (stale Custom|Sprint _output_get)))

(event Custom|Run
  (Variables|Default|SetMovementSpeed 3e+02)
  (Variables|/Script/Engine.CharacterMovementComponent|SetMaxWalkSpeed (Variables|Character|GetCharacterMovement) (stale Custom|Sprint _output_get)))

(event Custom|Sprint
  (bind _output_get (Variables|Default|SetMovementSpeed 375.0))
  (Variables|/Script/Engine.CharacterMovementComponent|SetMaxWalkSpeed (Variables|Character|GetCharacterMovement) _output_get))

(fn ConstructionScript)

(fn SetNewMoveSpeed
  (params (NewSpeed :type Float%20%28single-precision%29))
  (Variables|/Script/Engine.CharacterMovementComponent|SetMaxWalkSpeed (Variables|Character|GetCharacterMovement) NewSpeed))