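; Behavior tree task that sends the Servbot's controlled pawn toward an actor stored in a blackboard key.
; On execute it caches the Servbot AI controller, casting the owner on first use, and issues an AI MoveTo.
; The MoveTo's immediate output then updates the Servbot's move speed to a faster fixed value and finishes the task successfully, without waiting for arrival.
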(event EventReceiveExecute
  (params (OwnerActor :type Actor%20Object%20Reference))
  (if (!= (Variables|Default|GetAIConRef) 0)
    _
    (else
      (bind _asservbot_aicon_bp (Utilities|Casting|CastToServbot_AICon_BP OwnerActor))
      (bind _output_get (Variables|Default|SetAIConRef _asservbot_aicon_bp))))
  (AI|AIMoveTo (Pawn|GetControlledPawn _output_get) "0, 0, 0" (AI|BehaviorTree|GetBlackboardValueasActor (Variables|Default|GetTargetActorKey)) 5.0 false
    (:then
      (Default|UpdateMoveSpeed (Variables|/Game/Character/ServBot/Blueprints/AI/Servbot_AICon_BP.Servbot_AICon_BP_C|GetThisServbot _output_get) 375.0)
      (AI|BehaviorTree|FinishExecute true))))