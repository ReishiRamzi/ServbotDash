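; Behavior tree decorator for the ServBot AI that gates a branch on the pawn's distance to a target actor.
; It casts the owner to the ServBot AI controller, caches it, and reads the target actor from a blackboard key.
; Despite the CloseEnough name, it passes when that distance is at or beyond AcceptableDistance.
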(fn PerformConditionCheckAI
  (params (OwnerController :type AI%20Controller%20Object%20Reference) (ControlledPawn :type Pawn%20Object%20Reference))
  (bind _asservbot_aicon_bp (Utilities|Casting|CastToServbot_AICon_BP OwnerController))
  (Variables|Default|SetAIConRef _asservbot_aicon_bp)
  (return (>= (Math|Vector|VectorLength (- (Transformation|GetActorLocation (AI|BehaviorTree|GetBlackboardValueasActor (Variables|Default|GetTargetActorKey))) (Transformation|GetActorLocation (Pawn|GetControlledPawn (Variables|Default|GetAIConRef))))) (Variables|Default|GetAcceptableDistance))))